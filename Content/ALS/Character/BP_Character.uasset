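; Player character Blueprint with Enhanced Input move and look, weapon switching, aiming, and debug slow-motion keys.
; Weapon switching sets the equipped weapon and links the matching unarmed, gun or sword anim class layer onto the mesh.
; Aim press and release call UpdateGate, which passes the gate to the AnimInstance and applies that gate's speed, acceleration and braking values from the GateSettings map to CharacterMovement.
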(event Input|EnhancedActionEvents|EnhancedInputActionIA_SwitchWeapon
  (params (ActionValue :type Float%20%28double-precision%29) (ElapsedSeconds :type Float%20%28double-precision%29) (TriggeredSeconds :type Float%20%28double-precision%29) (InputAction :type Input%20Action%20Object%20Reference :default "/Game/ALS/Inputs/InputActions/IA_SwitchWeapon.IA_SwitchWeapon"))
  (bind _mesh (Variables|Character|GetMesh))
  ;[0.07708 0.7479 1] Switch Weapon event
  (:Started
    (switch int (Math|Float|Truncate ActionValue)
      (:1
        (Variables|Weapon|SetEquippedWeapon "NewEnumerator0")
        (Components|SkeletalMesh|AnimationBlueprintLinking|LinkAnimClassLayers _mesh "/Game/ALS/AnimationBlueprints/ABP_UnArmed.ABP_UnArmed_C"))
      (:2
        (Variables|Weapon|SetEquippedWeapon "NewEnumerator1")
        (Components|SkeletalMesh|AnimationBlueprintLinking|LinkAnimClassLayers _mesh "/Game/ALS/AnimationBlueprints/ABP_Gun.ABP_Gun_C"))
      (:3
        (Variables|Weapon|SetEquippedWeapon "NewEnumerator2")
        (Components|SkeletalMesh|AnimationBlueprintLinking|LinkAnimClassLayers _mesh "/Game/ALS/AnimationBlueprints/ABP_Sword.ABP_Sword_C")))))

(event Input|EnhancedActionEvents|EnhancedInputActionIA_Look
  (params (ActionValue :type Vector%202D%20Structure) (ElapsedSeconds :type Float%20%28double-precision%29) (TriggeredSeconds :type Float%20%28double-precision%29) (InputAction :type Input%20Action%20Object%20Reference :default "/Game/ALS/Inputs/InputActions/IA_Look.IA_Look"))
  (bind (_x _y) (Math|Vector2D|BreakVector2D ActionValue))
  ;[0.07708 0.7479 1] Looking around
  (Pawn|Input|AddControllerYawInput _x)
  (Pawn|Input|AddControllerPitchInput _y))

(event Input|EnhancedActionEvents|EnhancedInputActionIA_Move
  (params (ActionValue :type Vector%202D%20Structure) (ElapsedSeconds :type Float%20%28double-precision%29) (TriggeredSeconds :type Float%20%28double-precision%29) (InputAction :type Input%20Action%20Object%20Reference :default "/Game/ALS/Inputs/InputActions/IA_Move.IA_Move"))
  (bind (_x _y) (Math|Vector2D|BreakVector2D ActionValue))
  (bind _returnvalue (Pawn|GetControlRotation :!class /Script/Engine.Pawn))
  ;[0.07708 0.7479 1] Movement
  (Pawn|Input|AddMovementInput (Math|Vector|GetRightVector (Math|Rotator|MakeRotator (.roll _returnvalue) 0.0 (.yaw _returnvalue))) _x false)
  (Pawn|Input|AddMovementInput (Math|Vector|GetForwardVector (Math|Rotator|MakeRotator 0.0 0.0 (.yaw (Pawn|GetControlRotation :!class /Script/Engine.Pawn)))) _y false))

(event Input|EnhancedActionEvents|EnhancedInputActionIA_Aim
  (params (ActionValue :type Boolean) (ElapsedSeconds :type Float%20%28double-precision%29) (TriggeredSeconds :type Float%20%28double-precision%29) (InputAction :type Input%20Action%20Object%20Reference :default "/Game/ALS/Inputs/InputActions/IA_Aim.IA_Aim"))
  (:Started
    (CallFunction|UpdateGate "NewEnumerator0"))
  (:Completed
    (CallFunction|UpdateGate "NewEnumerator1")))

(event EventBeginPlay
  ;[0.1227 1 0.3772] Begin play init
  (bind _asplayer_controller (Utilities|Casting|CastToPlayerController (Pawn|GetController)))
  (Input|AddMappingContext (PlayerController|LocalPlayerSubsystems|GetEnhancedInputLocalPlayerSubsystem _asplayer_controller) "/Game/ALS/Inputs/IMC_ALS.IMC_ALS" 0 "(bIgnoreAllPressedKeysUntilRelease=True,bForceImmediately=False,bNotifyUserSettings=False)")
  (Components|SkeletalMesh|AnimationBlueprintLinking|LinkAnimClassLayers (Variables|Character|GetMesh) "/Game/ALS/AnimationBlueprints/ABP_UnArmed.ABP_UnArmed_C"))

(event Collision|EventActorBeginOverlap
  (params (OtherActor :type Actor%20Object%20Reference)))

(event EventTick
  (params (DeltaSeconds :type Float%20%28single-precision%29)))

(event Input|KeyboardEvents|DebugKeySubtract
  (params (Key :type Key%20Structure :default "None") (ActionValue :type Input%20Action%20Value%20Structure))
  (:Pressed
    (Utilities|Time|SetGlobalTimeDilation 0.1)))

(event Input|KeyboardEvents|DebugKeyAdd
  (params (Key :type Key%20Structure :default "None") (ActionValue :type Input%20Action%20Value%20Structure))
  (:Pressed
    (Utilities|Time|SetGlobalTimeDilation 1.0)))

(fn ConstructionScript)

(fn UpdateGate
  (params (Gate :type E_Gate%20Enum :default "NewEnumerator0"))
  (bind _gatesettings (Variables|Default|GetGateSettings))
  (bind _value (Utilities|Map|Find _gatesettings Gate))
  (bind (_maxwalkspeed _maxacceleration _brakingdeceleration _brakingfrictionfactor _brakingfriction _useseperatebrakingfiction) (Utilities|Struct|BreakS_GateSetting _value))
  (Variables|Default|SetCurrentGate Gate)
  (Class|BPIAnimationBlueprintInterface|RecieveCurrentGate(Message) (Components|SkeletalMesh|GetAnimInstance (Variables|Character|GetMesh)) Gate)
  (Utilities|FlowControl|Sequence
    (:then_0
      (Variables|/Script/Engine.CharacterMovementComponent|SetMaxWalkSpeed (Variables|Character|GetCharacterMovement) _maxwalkspeed))
    (:then_1
      (Variables|/Script/Engine.CharacterMovementComponent|SetMaxAcceleration (Variables|Character|GetCharacterMovement) _maxacceleration))
    (:then_2
      (Variables|/Script/Engine.CharacterMovementComponent|SetBrakingDecelerationWalking (Variables|Character|GetCharacterMovement) _brakingdeceleration))
    (:then_3
      (Variables|/Script/Engine.CharacterMovementComponent|SetBrakingFrictionFactor (Variables|Character|GetCharacterMovement) _brakingfrictionfactor))
    (:then_4
      (Variables|/Script/Engine.CharacterMovementComponent|SetBrakingFriction (Variables|Character|GetCharacterMovement) _brakingfriction))
    (:then_5
      (Variables|/Script/Engine.CharacterMovementComponent|SetbUseSeparateBrakingFriction (Variables|Character|GetCharacterMovement) _useseperatebrakingfiction))))